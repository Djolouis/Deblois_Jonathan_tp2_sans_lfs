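; Card verification spotlight for the extraterrestrial map, with custom events for a correct card (bonnecarte) and no card (pascarte).
; Both events run identical logic: two chained timed MoveComponentTo calls tilt the SpotLightComponent's pitch to near horizontal, then steeply downward.
; The moves feed the light's current world location, roll and yaw into relative-space targets.
; The file contains no card-checking logic.
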(event `bonne carte`
  (bind _spotlightcomponent (`self.SpotLightComponent`))
  (bind _spotlightcomponent_2 (`self.SpotLightComponent`))
  (bind (_returnvalue_roll _returnvalue_pitch _returnvalue_yaw) (`KismetMathLibrary.BreakRotator` (`SceneComponent.K2_GetComponentRotation` _spotlightcomponent)))
  (bind (_returnvalue_roll_2 _returnvalue_pitch_2 _returnvalue_yaw_2) (`KismetMathLibrary.BreakRotator` (`SceneComponent.K2_GetComponentRotation` _spotlightcomponent_2)))
  ; s bonne carte
  (`KismetSystemLibrary.MoveComponentTo` _spotlightcomponent (`SceneComponent.K2_GetComponentLocation` _spotlightcomponent) (`KismetMathLibrary.MakeRotator` _returnvalue_roll -4.0 _returnvalue_yaw) false false 2.0)
  (`KismetSystemLibrary.MoveComponentTo` _spotlightcomponent_2 (`SceneComponent.K2_GetComponentLocation` _spotlightcomponent_2) (`KismetMathLibrary.MakeRotator` _returnvalue_roll_2 -82.0 _returnvalue_yaw_2) false false 2.0))

(event `pas carte`
  (bind _spotlightcomponent (`self.SpotLightComponent`))
  (bind _spotlightcomponent_2 (`self.SpotLightComponent`))
  (bind (_returnvalue_roll _returnvalue_pitch _returnvalue_yaw) (`KismetMathLibrary.BreakRotator` (`SceneComponent.K2_GetComponentRotation` _spotlightcomponent_2)))
  (bind (_returnvalue_roll_2 _returnvalue_pitch_2 _returnvalue_yaw_2) (`KismetMathLibrary.BreakRotator` (`SceneComponent.K2_GetComponentRotation` _spotlightcomponent)))
  ; s bonne carte
  (`KismetSystemLibrary.MoveComponentTo` _spotlightcomponent_2 (`SceneComponent.K2_GetComponentLocation` _spotlightcomponent_2) (`KismetMathLibrary.MakeRotator` _returnvalue_roll -4.0 _returnvalue_yaw) false false 2.0)
  (`KismetSystemLibrary.MoveComponentTo` _spotlightcomponent (`SceneComponent.K2_GetComponentLocation` _spotlightcomponent) (`KismetMathLibrary.MakeRotator` _returnvalue_roll_2 -82.0 _returnvalue_yaw_2) false false 2.0))

(fn `UserConstructionScript`)